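; Car hazard actor that drives along a SplineRoad and kills the third-person player character on hit.
; After a delay on BeginPlay, it finds the road and runs a timeline that lerps position along the spline, with rotation fixed to the spline's start.
; A one-time proximity check can play driving audio.
; Hits call CharDeath, play impact and dying sounds, and show the Death widget.
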(event Custom|Move%20Object
  (bind _spline_ref (Variables|Default|GetSpline%20Ref))
  (bind _spline (Variables|/Game/SplineRoad.SplineRoad_C|GetSpline _spline_ref))
  (Components|Timeline|SetPlayRate (Variables|Default|GetMove%20Object%20T) (/ 1.0 (Variables|Default|GetTime%20To%20Complete%20%28secs%29)))
  (bind _move_track (Timeline|Move%20Object%20T Play)
    (:Update
      (Transformation|SetActorTransform (Math|Transform|MakeTransform (Spline|GetLocationatDistanceAlongSpline _spline (Math|Float|Lerp 0.0 (Spline|GetSplineLength (Variables|/Game/SplineRoad.SplineRoad_C|GetSpline (Variables|Default|GetSpline%20Ref))) _move_track) "World") (Spline|GetRotationatDistanceAlongSpline _spline 0.0 "Local") "1,1,1")))))

(event EventBeginPlay
  (Utilities|FlowControl|Delay (Variables|Default|Getdelay))
  (bind _returnvalue (Actor|GetActorOfClass "/Game/SplineRoad.SplineRoad_C"))
  (Variables|Default|SetSpline%20Ref _returnvalue)
  (CallFunction|MoveObject)
  (if (< (Transformation|GetDistanceTo (Game|Player|GetPlayerPawn 0)) 2e+02)
    (Audio|PlaySoundatLocation "/Game/Audio/EnvironmentalSounds/cars_driving.cars_driving" "0, 0, 0" "0, 0, 0" 1.0 1.0 0.0 0 0 0)))

(event Collision|EventHit
  (params (MyComp :type Primitive%20Component%20Object%20Reference) (Other :type Actor%20Object%20Reference) (OtherComp :type Primitive%20Component%20Object%20Reference) (bSelfMoved :type Boolean) (HitLocation :type Vector :default "0, 0, 0") (HitNormal :type Vector :default "0, 0, 0") (NormalImpulse :type Vector :default "0, 0, 0") (Hit :type Hit%20Result%20Structure%20%28by%20ref%29))
  (bind _returnvalue (Components|GetOwner OtherComp))
  (if (== (Utilities|GetClass _returnvalue) "/Game/ThirdPersonCharacter.ThirdPersonCharacter_C")
    (bind _asthird_person_character (Utilities|Casting|CastToThirdPersonCharacter _returnvalue))
    (Default|CharDeath _asthird_person_character)
    (Audio|PlaySoundatLocation "/Game/Audio/EnvironmentalSounds/hit_by_car.hit_by_car" (Transformation|GetActorLocation _asthird_person_character) "0, 0, 0" 1.0 1.0 0.0 0 0 0)
    (Utilities|FlowControl|Delay 0.3)
    (Audio|PlaySoundatLocation "/Game/Audio/CreatureSounds/Skeebo/raccoon_dying.raccoon_dying" "0, 0, 0" "0, 0, 0" 1.0 1.0 0.0 0 0 0)
    (bind _returnvalue_2 (UserInterface|CreateWidget "/Game/UI/Death.Death_C"))
    (UserInterface|Viewport|AddtoViewport _returnvalue_2 0)))

(fn ConstructionScript)