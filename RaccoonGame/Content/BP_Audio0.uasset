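; BP_Audio0 is an audio actor that plays a raccoon scream tied to the player character's Off flag.
; Each Tick it casts the player pawn to ThirdPersonCharacter and, while Off is true, adds the audio component once through a DoOnce.
; When Off is false it stops the scream and destroys itself.
; A separate Off event resets the DoOnce.
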(event Custom|Off
  (Utilities|FlowControl|DoOnce false) ; enters at Reset
)

(event EventTick
  (params (DeltaSeconds :type Float%20%28single-precision%29))
  (if (Variables|/Game/ThirdPersonCharacter.ThirdPersonCharacter_C|GetbOff (.AsThird%20Person%20Character (Utilities|Casting|CastToThirdPersonCharacter (Game|Player|GetPlayerPawn 0))))
    (Utilities|FlowControl|DoOnce false
      (:Completed
        (bind _returnvalue (AddComponent|AddAudioComponent false))
        (Variables|Default|SetRaccoon%20scream _returnvalue)))
    (else
      (Audio|Components|Audio|Stop (Variables|Default|GetRaccoon%20scream))
      (Actor|DestroyActor))))

(fn ConstructionScript)