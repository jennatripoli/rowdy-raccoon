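; Base NPC Blueprint that follows a daily schedule driven by the SunSky solar time and reacts to player proximity.
; A looping delay re-checks state, switching on the hour to send the NPC via AI navigation to random points around its Spot, Food or Bed locations.
; It hides at bedtime, with no unhide in this graph.
; A nearby player overrides the schedule, sending it to a random reachable point around itself.
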(event Custom|isAsleep
  (bind _self self)
  (bind _nav_data (Variables|Default|GetNav%20Data))
  (bind _returnvalue (AI|GetAIController _self))
  ;[1 1 1] Proximity detection
  (Utilities|FlowControl|Delay 0.2)
  (if (< (Transformation|GetDistanceTo (Game|Player|GetPlayerPawn 0)) 5e+02)
    ;[1 1 1] Daily Schedule
    (CallFunction|IsClose)
    (else
      (switch int (Math|Integer|%(Integer) (Math|Float|Round (Variables|/SunPosition/SunSky.SunSky_C|GetSolarTime (stale EventBeginPlay _output_get))) 24)
        (:0
          (CallFunction|IsAsleep :!label _label))
        (:1
          (goto _label))
        (:2
          (goto _label))
        (:3
          (goto _label))
        (:4
          (goto _label))
        (:5
          (goto _label))
        (:6
          (goto _label))
        (:7
          (AI|Navigation|SimpleMovetoLocation _returnvalue (.RandomLocation (AI|Navigation|GetRandomReachablePointinRadius (Variables|Default|Getspot) 3e+02 _nav_data 0)) :!label _label_2)
          (CallFunction|IsWaiting :!label _label_3))
        (:8
          (goto _label_3))
        (:9
          (goto _label_3))
        (:10
          (goto _label_3))
        (:11
          (goto _label_3))
        (:12
          (AI|Navigation|SimpleMovetoLocation _returnvalue (.RandomLocation (AI|Navigation|GetRandomReachablePointinRadius (Variables|Default|Getfood) 3e+02 _nav_data 0)))
          (goto _label_3))
        (:13
          (goto _label_2))
        (:14
          (goto _label_3))
        (:15
          (goto _label_3))
        (:16
          (goto _label_3))
        (:17
          (goto _label_3))
        (:18
          (AI|Navigation|SimpleMovetoLocation _returnvalue (.RandomLocation (AI|Navigation|GetRandomReachablePointinRadius (Variables|Default|Getbed) 3e+02 _nav_data 0)))
          (Rendering|SetActorHiddenInGame true)
          (goto _label))
        (:19
          (goto _label))
        (:20
          (goto _label))
        (:21
          (goto _label))
        (:22
          (goto _label))
        (:23
          (goto _label))))))

(event Custom|isWaiting
  (bind _self self)
  (bind _nav_data (Variables|Default|GetNav%20Data))
  (bind _returnvalue (AI|GetAIController _self))
  ;[1 1 1] Proximity detection
  (Utilities|FlowControl|Delay 0.2)
  (if (< (Transformation|GetDistanceTo (Game|Player|GetPlayerPawn 0)) 5e+02)
    ;[1 1 1] Daily Schedule
    (CallFunction|IsClose)
    (else
      (switch int (Math|Integer|%(Integer) (Math|Float|Round (Variables|/SunPosition/SunSky.SunSky_C|GetSolarTime (stale EventBeginPlay _output_get))) 24)
        (:0
          (CallFunction|IsAsleep :!label _label))
        (:1
          (goto _label))
        (:2
          (goto _label))
        (:3
          (goto _label))
        (:4
          (goto _label))
        (:5
          (goto _label))
        (:6
          (goto _label))
        (:7
          (AI|Navigation|SimpleMovetoLocation _returnvalue (.RandomLocation (AI|Navigation|GetRandomReachablePointinRadius (Variables|Default|Getspot) 3e+02 _nav_data 0)) :!label _label_2)
          (CallFunction|IsWaiting :!label _label_3))
        (:8
          (goto _label_3))
        (:9
          (goto _label_3))
        (:10
          (goto _label_3))
        (:11
          (goto _label_3))
        (:12
          (AI|Navigation|SimpleMovetoLocation _returnvalue (.RandomLocation (AI|Navigation|GetRandomReachablePointinRadius (Variables|Default|Getfood) 3e+02 _nav_data 0)))
          (goto _label_3))
        (:13
          (goto _label_2))
        (:14
          (goto _label_3))
        (:15
          (goto _label_3))
        (:16
          (goto _label_3))
        (:17
          (goto _label_3))
        (:18
          (AI|Navigation|SimpleMovetoLocation _returnvalue (.RandomLocation (AI|Navigation|GetRandomReachablePointinRadius (Variables|Default|Getbed) 3e+02 _nav_data 0)))
          (Rendering|SetActorHiddenInGame true)
          (goto _label))
        (:19
          (goto _label))
        (:20
          (goto _label))
        (:21
          (goto _label))
        (:22
          (goto _label))
        (:23
          (goto _label))))))

(event Custom|isClose
  ;[1 1 1] Panic state
  (AI|Navigation|SimpleMovetoLocation (AI|GetAIController self) (.RandomLocation (AI|Navigation|GetRandomReachablePointinRadius (Transformation|GetActorLocation) 2e+03 (Variables|Default|GetNav%20Data) 0)))
  (Utilities|FlowControl|Delay 1.2)
  (CallFunction|IsWaiting))

(event EventTick
  (params (DeltaSeconds :type Float%20%28single-precision%29))
  ;[1 1 1] Panic state
)

(event EventBeginPlay
  (bind _self self)
  (bind _returnvalue (AI|GetAIController _self))
  ;[1 1 1] Praise the Sun
  (bind _returnvalue_2 (Actor|GetActorOfClass "/SunPosition/SunSky.SunSky_C"))
  (bind _output_get (Variables|Default|Setsun _returnvalue_2))
  (bind _returnvalue_3 (Actor|GetActorOfClass "/Script/NavigationSystem.RecastNavMesh"))
  (Variables|Default|SetNav%20Data _returnvalue_3)
  ;[1 1 1] Proximity detection
  (if (< (Transformation|GetDistanceTo (Game|Player|GetPlayerPawn 0)) 5e+02)
    ;[1 1 1] Daily Schedule
    (CallFunction|IsClose)
    (else
      (switch int (Math|Integer|%(Integer) (Math|Float|Round (Variables|/SunPosition/SunSky.SunSky_C|GetSolarTime _output_get)) 24)
        (:0
          (CallFunction|IsAsleep :!label _label))
        (:1
          (goto _label))
        (:2
          (goto _label))
        (:3
          (goto _label))
        (:4
          (goto _label))
        (:5
          (goto _label))
        (:6
          (goto _label))
        (:7
          (AI|Navigation|SimpleMovetoLocation _returnvalue (.RandomLocation (AI|Navigation|GetRandomReachablePointinRadius (Variables|Default|Getspot) 3e+02 (Variables|Default|GetNav%20Data) 0)) :!label _label_2)
          (CallFunction|IsWaiting :!label _label_3))
        (:8
          (goto _label_3))
        (:9
          (goto _label_3))
        (:10
          (goto _label_3))
        (:11
          (goto _label_3))
        (:12
          (AI|Navigation|SimpleMovetoLocation _returnvalue (.RandomLocation (AI|Navigation|GetRandomReachablePointinRadius (Variables|Default|Getfood) 3e+02 (Variables|Default|GetNav%20Data) 0)))
          (goto _label_3))
        (:13
          (goto _label_2))
        (:14
          (goto _label_3))
        (:15
          (goto _label_3))
        (:16
          (goto _label_3))
        (:17
          (goto _label_3))
        (:18
          (AI|Navigation|SimpleMovetoLocation _returnvalue (.RandomLocation (AI|Navigation|GetRandomReachablePointinRadius (Variables|Default|Getbed) 3e+02 (Variables|Default|GetNav%20Data) 0)))
          (Rendering|SetActorHiddenInGame true)
          (goto _label))
        (:19
          (goto _label))
        (:20
          (goto _label))
        (:21
          (goto _label))
        (:22
          (goto _label))
        (:23
          (goto _label))))))

(fn ConstructionScript)