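; Base NPC AI controller that runs a daily routine driven by the SunSky solar time.
; The rounded hour picks moves to a work spot, lunch or bed, or idle waiting and sleep, hiding the character on reaching bed.
; A player within 500 units overrides the schedule with a move to a random reachable point.
; Waiting and sleep events re-run the checks after a short delay, forming a polling loop.
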(event Custom|IsClose
  (bind _returnvalue (Pawn|GetControlledPawn))
  ;[1 1 1] Panic state
  (AI|AIMoveTo _returnvalue (.RandomLocation (AI|Navigation|GetRandomReachablePointinRadius (Transformation|GetActorLocation _returnvalue) 2e+03 0 0)) 0 5.0 false
    (:OnSuccess
      (AI|Navigation|StopMovement)
      (CallFunction|IsWaiting))))

(event Custom|isAsleep
  (bind _returnvalue (Pawn|GetControlledPawn))
  ;[1 1 1] Proximity detection
  (Utilities|FlowControl|Delay 0.2)
  (if (< (Transformation|GetDistanceTo (Pawn|GetControlledPawn) (Game|Player|GetPlayerPawn 0)) 5e+02)
    (CallFunction|IsClose)
    (else
      ;[1 1 1] Daily Schedule
      (switch int (Math|Integer|%(Integer) (Math|Float|Round (Variables|/SunPosition/SunSky.SunSky_C|GetSolarTime (stale EventBeginPlay _output_get))) 24)
        (:0
          (CallFunction|IsAsleep :!label _label))
        (:1
          (goto _label))
        (:2
          (goto _label))
        (:3
          (goto _label))
        (:4
          (goto _label))
        (:5
          (goto _label))
        (:6
          (goto _label))
        (:7
          (AI|AIMoveTo _returnvalue (Variables|Default|Getspot) 0 5e+02 false :!label _label_2 ; waking up
            (:OnSuccess
              (CallFunction|IsWaiting :!label _label_3))))
        (:8
          (goto _label_3))
        (:9
          (goto _label_3))
        (:10
          (goto _label_3))
        (:11
          (goto _label_3))
        (:12
          (AI|AIMoveTo _returnvalue (Variables|Default|Getfood) 0 5e+02 false ; lunchtime
            (:OnSuccess
              (goto _label_3))))
        (:13
          (goto _label_2))
        (:14
          (goto _label_3))
        (:15
          (goto _label_3))
        (:16
          (goto _label_3))
        (:17
          (goto _label_3))
        (:18
          (AI|AIMoveTo _returnvalue (Variables|Default|Getbed) 0 3e+02 false ; going home
            (:OnSuccess
              (bind _asthird_person_character (Utilities|Casting|CastToThirdPersonCharacter (Pawn|GetControlledPawn)))
              (Rendering|SetActorHiddenInGame _asthird_person_character true)
              (goto _label))))
        (:19
          (goto _label))
        (:20
          (goto _label))
        (:21
          (goto _label))
        (:22
          (goto _label))
        (:23
          (goto _label))))))

(event Custom|isWaiting
  (bind _returnvalue (Pawn|GetControlledPawn))
  ;[1 1 1] Proximity detection
  (Utilities|FlowControl|Delay 0.2)
  (if (< (Transformation|GetDistanceTo (Pawn|GetControlledPawn) (Game|Player|GetPlayerPawn 0)) 5e+02)
    (CallFunction|IsClose)
    (else
      ;[1 1 1] Daily Schedule
      (switch int (Math|Integer|%(Integer) (Math|Float|Round (Variables|/SunPosition/SunSky.SunSky_C|GetSolarTime (stale EventBeginPlay _output_get))) 24)
        (:0
          (CallFunction|IsAsleep :!label _label))
        (:1
          (goto _label))
        (:2
          (goto _label))
        (:3
          (goto _label))
        (:4
          (goto _label))
        (:5
          (goto _label))
        (:6
          (goto _label))
        (:7
          (AI|AIMoveTo _returnvalue (Variables|Default|Getspot) 0 5e+02 false :!label _label_2 ; waking up
            (:OnSuccess
              (CallFunction|IsWaiting :!label _label_3))))
        (:8
          (goto _label_3))
        (:9
          (goto _label_3))
        (:10
          (goto _label_3))
        (:11
          (goto _label_3))
        (:12
          (AI|AIMoveTo _returnvalue (Variables|Default|Getfood) 0 5e+02 false ; lunchtime
            (:OnSuccess
              (goto _label_3))))
        (:13
          (goto _label_2))
        (:14
          (goto _label_3))
        (:15
          (goto _label_3))
        (:16
          (goto _label_3))
        (:17
          (goto _label_3))
        (:18
          (AI|AIMoveTo _returnvalue (Variables|Default|Getbed) 0 3e+02 false ; going home
            (:OnSuccess
              (bind _asthird_person_character (Utilities|Casting|CastToThirdPersonCharacter (Pawn|GetControlledPawn)))
              (Rendering|SetActorHiddenInGame _asthird_person_character true)
              (goto _label))))
        (:19
          (goto _label))
        (:20
          (goto _label))
        (:21
          (goto _label))
        (:22
          (goto _label))
        (:23
          (goto _label))))))

(event EventBeginPlay
  (bind _returnvalue (Pawn|GetControlledPawn))
  ;[1 1 1] Praise the Sun
  (bind _returnvalue_2 (Actor|GetActorOfClass "/SunPosition/SunSky.SunSky_C"))
  (bind _output_get (Variables|Default|Setsun _returnvalue_2))
  ;[1 1 1] Proximity detection
  (if (< (Transformation|GetDistanceTo (Pawn|GetControlledPawn) (Game|Player|GetPlayerPawn 0)) 5e+02)
    (CallFunction|IsClose)
    (else
      ;[1 1 1] Daily Schedule
      (switch int (Math|Integer|%(Integer) (Math|Float|Round (Variables|/SunPosition/SunSky.SunSky_C|GetSolarTime _output_get)) 24)
        (:0
          (CallFunction|IsAsleep :!label _label))
        (:1
          (goto _label))
        (:2
          (goto _label))
        (:3
          (goto _label))
        (:4
          (goto _label))
        (:5
          (goto _label))
        (:6
          (goto _label))
        (:7
          (AI|AIMoveTo _returnvalue (Variables|Default|Getspot) 0 5e+02 false :!label _label_2 ; waking up
            (:OnSuccess
              (CallFunction|IsWaiting :!label _label_3))))
        (:8
          (goto _label_3))
        (:9
          (goto _label_3))
        (:10
          (goto _label_3))
        (:11
          (goto _label_3))
        (:12
          (AI|AIMoveTo _returnvalue (Variables|Default|Getfood) 0 5e+02 false ; lunchtime
            (:OnSuccess
              (goto _label_3))))
        (:13
          (goto _label_2))
        (:14
          (goto _label_3))
        (:15
          (goto _label_3))
        (:16
          (goto _label_3))
        (:17
          (goto _label_3))
        (:18
          (AI|AIMoveTo _returnvalue (Variables|Default|Getbed) 0 3e+02 false ; going home
            (:OnSuccess
              (bind _asthird_person_character (Utilities|Casting|CastToThirdPersonCharacter (Pawn|GetControlledPawn)))
              (Rendering|SetActorHiddenInGame _asthird_person_character true)
              (goto _label))))
        (:19
          (goto _label))
        (:20
          (goto _label))
        (:21
          (goto _label))
        (:22
          (goto _label))
        (:23
          (goto _label))))))

(fn ConstructionScript)